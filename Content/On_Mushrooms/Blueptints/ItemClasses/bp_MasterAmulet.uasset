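; Base amulet item Blueprint that equips itself on the top-down player character when used.
; On BeginPlay it caches the first My_TopDownCharacter in the level and that character's cage reference.
; The use event passes the amulet to EquipAmulet on the character, reached through its Cage reference.
; StopInfluence is an empty event, and the construction script only calls its parent.
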(event Custom|StopInfluence)

(event EventBeginPlay
  (bind _outactors (Actor|GetAllActorsOfClass "/Game/On_Mushrooms/Character/My_TopDownCharacter.My_TopDownCharacter_C"))
  (bind _output_get (Variables|Default|SetTopDownCharacterReference (Utilities|Array|Get(acopy) _outactors)))
  (Variables|Default|SetCage%20Ref (Variables|/Game/On_Mushrooms/Character/My_TopDownCharacter.My_TopDownCharacter_C|GetCageRef _output_get)))

(event Collision|EventActorBeginOverlap
  (params (OtherActor :type Actor%20Object%20Reference)))

(event EventTick
  (params (DeltaSeconds :type Float%20%28single-precision%29)))

(event EventEventonUsed
  (Default|-EquipAmulet (Variables|/Game/On_Mushrooms/Blueptints/UI/bp_Cage.bp_Cage_C|GetTopDownCharReference (Variables|Default|GetCage)) self))

(fn ConstructionScript
  (|CallParentFunction))