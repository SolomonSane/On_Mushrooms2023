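; Speed amulet item that temporarily raises the top-down character's max speed when used.
; On use it asks the character to equip it and, if that succeeds, applies the speed increase and waits for its duration.
; It then unequips the amulet and calls the character's OnoverloadedEnd.
; StopInfluence calls OnoverloadedEnd directly, skipping the unequip, without cancelling the pending delay.
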(event EventBeginPlay
  (|CallParentFunction) ; This node is disabled and will not be called.\nDrag off pins to build functionality.
)

(event Collision|EventActorBeginOverlap
  (params (OtherActor :type Actor%20Object%20Reference))
  (|CallParentFunction OtherActor) ; This node is disabled and will not be called.\nDrag off pins to build functionality.
)

(event EventEventonUsed
  (bind _success (Default|-EquipAmulet (Variables|/Game/On_Mushrooms/Blueptints/UI/bp_Cage.bp_Cage_C|GetTopDownCharReference (Variables|Default|GetCage%20Ref)) self))
  (if _success
    (Default|-IncreaseMaxSpeed (Variables|Default|GetTopDownCharacterReference))
    (Utilities|FlowControl|Delay (Variables|Default|GetDuration))
    (Default|-UnequipAmulet (Variables|Default|GetTopDownCharacterReference) false)
    (Default|-OnoverloadedEnd (Variables|Default|GetTopDownCharacterReference))))

(event EventStopInfluence
  (Default|-OnoverloadedEnd (Variables|Default|GetTopDownCharacterReference)))

(fn ConstructionScript
  (|CallParentFunction))