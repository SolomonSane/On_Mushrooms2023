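; Master item Blueprint for a usable, hoverable item tied to the faery spawner that owns it.
; Cursor hover toggles its SpiderWeb component and notifies the spawner, using a ward-specific hover call when the spawner's item-class Humor matches the RolledHumor in the player's cage.
; On use, it removes one unit at its index from the Cage and destroys itself if that succeeds.
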(event OnBeginCursorOver(StaticMesh)
  (params (TouchedComponent :type Primitive%20Component%20Object%20Reference))
  (Rendering|SetVisibility (Variables|Default|GetSpiderWeb) true false)
  (if (Utilities|Enum|Equal(Enum) (Utilities|Struct|Breaks_ItemInfo (Utilities|GetClassDefaults (Variables|/Game/On_Mushrooms/Blueptints/ItemClasses/bp_Faery_Spawner.bp_Faery_Spawner_C|GetItem%20Class (stale EventBeginPlay _output_get)))) (Variables|/Game/On_Mushrooms/Blueptints/UI/bp_Cage.bp_Cage_C|GetRolledHumor (Variables|/Game/On_Mushrooms/Character/My_TopDownCharacter.My_TopDownCharacter_C|GetCageRef (.AsMy%20Top%20Down%20Character (Utilities|Casting|CastToMy_TopDownCharacter (Game|Player|GetPlayerPawn 0))))))
    (Default|-onHoveredtoWard (stale EventBeginPlay _output_get))
    (else
      (Default|-onHovered (stale EventBeginPlay _output_get)))))

(event OnEndCursorOver(StaticMesh)
  (params (TouchedComponent :type Primitive%20Component%20Object%20Reference))
  (Rendering|SetVisibility (Variables|Default|GetSpiderWeb) false false)
  (Default|-onUnhovered (stale EventBeginPlay _output_get)))

(event Custom|EventOnUsed
  (bind _success_ (Default|-RemoveItematIndex (Variables|Default|GetCage) (Variables|OnSpawn(непутатьсfaerySpawn)|GetIndex) 1 false))
  (if _success_
    (Actor|DestroyActor)))

(event EventBeginPlay
  (Rendering|SetVisibility (Variables|Default|GetSpiderWeb) false false)
  (bind _asbp_faery_spawner (Utilities|Casting|CastTobp_Faery_Spawner (Components|GetOwner)))
  (bind _output_get (Variables|Default|SetFaerySpawner _asbp_faery_spawner)))

(fn ConstructionScript)