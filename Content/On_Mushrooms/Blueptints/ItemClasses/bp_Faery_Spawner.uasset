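; Pickup spawner that spawns a random item from SpawnedClasses and shows its name on a widget, colored by humor.
; Sphere overlaps maintain the character's NearbyPickupActors list, passing prompt visibility to the first entry.
; OnPickup spends stamina to add the item to the cage, while gold and stamina items grant fixed amounts directly.
; The spawned item is then destroyed, even if adding fails, and a replacement appears after a short delay.
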(event OnComponentBeginOverlap(SphereCollision)
  (params (OverlappedComponent :type Primitive%20Component%20Object%20Reference) (OtherActor :type Actor%20Object%20Reference) (OtherComp :type Primitive%20Component%20Object%20Reference) (OtherBodyIndex :type Integer) (bFromSweep :type Boolean) (SweepResult :type Hit%20Result%20Structure%20%28by%20ref%29))
  (bind _asmy_top_down_character (Utilities|Casting|CastToMy_TopDownCharacter OtherActor))
  (if (> (Utilities|Array|Length (Variables|/Game/On_Mushrooms/Character/My_TopDownCharacter.My_TopDownCharacter_C|GetNearbyPickupActors _asmy_top_down_character)) 0)
    (Utilities|Array|Add (Variables|/Game/On_Mushrooms/Character/My_TopDownCharacter.My_TopDownCharacter_C|GetNearbyPickupActors _asmy_top_down_character) self)
    (else
      (Rendering|SetVisibility (Variables|Default|GetPickupText) true false)
      (Utilities|Array|Add (Variables|/Game/On_Mushrooms/Character/My_TopDownCharacter.My_TopDownCharacter_C|GetNearbyPickupActors _asmy_top_down_character) self))))

(event OnComponentEndOverlap(SphereCollision)
  (params (OverlappedComponent :type Primitive%20Component%20Object%20Reference) (OtherActor :type Actor%20Object%20Reference) (OtherComp :type Primitive%20Component%20Object%20Reference) (OtherBodyIndex :type Integer))
  (bind _asmy_top_down_character (Utilities|Casting|CastToMy_TopDownCharacter OtherActor))
  (if (and (Utilities|IsValid (Utilities|Array|Get(acopy) (Variables|/Game/On_Mushrooms/Character/My_TopDownCharacter.My_TopDownCharacter_C|GetNearbyPickupActors _asmy_top_down_character))) (== (Utilities|Array|Get(acopy) (Variables|/Game/On_Mushrooms/Character/My_TopDownCharacter.My_TopDownCharacter_C|GetNearbyPickupActors _asmy_top_down_character)) self))
    (Rendering|SetVisibility (Variables|Default|GetPickupText) false false)
    (Utilities|Array|RemoveItem (Variables|/Game/On_Mushrooms/Character/My_TopDownCharacter.My_TopDownCharacter_C|GetNearbyPickupActors _asmy_top_down_character) self)
    (Utilities|IsValid (Utilities|Array|Get(acopy) (Variables|/Game/On_Mushrooms/Character/My_TopDownCharacter.My_TopDownCharacter_C|GetNearbyPickupActors _asmy_top_down_character))
      (:Is%20Valid
        (Rendering|SetVisibility (Variables|bp_Faery_Spawner_C|GetPickupText (Utilities|Array|Get(acopy) (Variables|/Game/On_Mushrooms/Character/My_TopDownCharacter.My_TopDownCharacter_C|GetNearbyPickupActors _asmy_top_down_character))) true false)))
    (else
      (Utilities|Array|RemoveItem (Variables|/Game/On_Mushrooms/Character/My_TopDownCharacter.My_TopDownCharacter_C|GetNearbyPickupActors _asmy_top_down_character) self))))

(event Custom|OnPickup
  (params (TopDownChar :type My%20Top%20Down%20Character%20Object%20Reference))
  (bind _nearbypickupactors (Variables|/Game/On_Mushrooms/Character/My_TopDownCharacter.My_TopDownCharacter_C|GetNearbyPickupActors TopDownChar))
  (bind _spawneditem (Variables|Default|GetSpawnedItem))
  (bind _output (Utilities|Array|Get(acopy) _nearbypickupactors))
  (if (and (!= (Variables|Default|GetItem%20Class) "/Game/On_Mushrooms/Blueptints/ItemClasses/bp_Gold.bp_Gold_C") (!= (Variables|Default|GetItem%20Class) "/Game/On_Mushrooms/Blueptints/ItemClasses/bp_Stamina.bp_Stamina_C"))
    (bind _output_get (Variables|Default|SetCage%20Ref (Variables|/Game/On_Mushrooms/Character/My_TopDownCharacter.My_TopDownCharacter_C|GetCageRef TopDownChar)))
    (Utilities|IsValid _output_get
      (:Is%20Valid
        (bind _newcosttodrag (Default|-IncreaseCosttoDrag (Variables|/Game/On_Mushrooms/Blueptints/UI/bp_Cage.bp_Cage_C|GetCage%20Widget (Variables|Default|GetCage%20Ref)) (Variables|Default|GetItem%20Class)))
        (if (>= (Variables|/Game/On_Mushrooms/Character/My_TopDownCharacter.My_TopDownCharacter_C|GetCurrentStamina (Variables|Default|GetTopDownCharacterReference)) _newcosttodrag)
          (Default|-DecreaseStamina (Variables|Default|GetTopDownCharacterReference) _newcosttodrag)
          (bind _success2 (Default|-AddItem (Variables|Default|GetCage%20Ref) (Variables|Default|GetItem%20Class) (Variables|Default|GetAmount) true))
          (if _success2
            (Utilities|Array|RemoveItem _nearbypickupactors self)
            (Utilities|IsValid _output
              (:Is%20Valid
                (Rendering|SetVisibility (Variables|bp_Faery_Spawner_C|GetPickupText _output) true false))
              (:Is%20Not%20Valid
                _)))
          (Utilities|IsValid _spawneditem :!label _label
            (:Is%20Valid
              (Actor|DestroyActor _spawneditem)
              (Utilities|FlowControl|Delay 3.0)
              (CallFunction|SpawnFaery)
              (CallFunction|-UpdateText))))))
    (elif (!= (Variables|Default|GetItem%20Class) "/Game/On_Mushrooms/Blueptints/ItemClasses/bp_Stamina.bp_Stamina_C")
      (Default|-IncreaseGold TopDownChar 5) ; В амаунте задаем количество золота за подъем монеты
      (goto _label)
      (else
        (Default|-IncreaseStamina TopDownChar 5) ; задаем количество за поднятие стамины
        (goto _label)))))

(event EventBeginPlay
  (bind _outactors (Actor|GetAllActorsOfClass "/Game/On_Mushrooms/Character/My_TopDownCharacter.My_TopDownCharacter_C"))
  (Variables|Default|SetTopDownCharacterReference (Utilities|Array|Get(acopy) _outactors))
  (CallFunction|SpawnFaery)
  (CallFunction|-UpdateText))

(event Collision|EventActorBeginOverlap
  (params (OtherActor :type Actor%20Object%20Reference)))

(event EventTick
  (params (DeltaSeconds :type Float%20%28single-precision%29)))

(fn ConstructionScript)

(fn SpawnFaery
  (bind _output_get (Variables|Default|SetItem%20Class (.OutItem (Utilities|Array|Random (Variables|Default|Getspawned_classes)))))
  (bind _returnvalue (Game|SpawnActorfromClass _output_get (Transformation|GetActorTransform) "AdjustIfPossibleButAlwaysSpawn" 0 (Variables|Default|GetCage%20Ref) 0 0))
  (Variables|Default|SetSpawnedItem _returnvalue))

(fn -UpdateText
  (bind _item_class (Variables|Default|GetItem%20Class))
  (bind _iteminfo (Utilities|GetClassDefaults _item_class))
  (bind (_name _humor) (Utilities|Struct|Breaks_ItemInfo _iteminfo))
  (bind _asw_pickup_text (Utilities|Casting|CastTow_PickupText (UserInterface|GetUserWidgetObject (Variables|Default|GetPickupText)))
    (:then
      (Rendering|Components|TextRender|SetText (Variables|/Game/On_Mushrooms/Widgets/w_PickupText.w_PickupText_C|GetNameText _asw_pickup_text) (Utilities|Text|FormatText _name))
      (Appearance|SetColorandOpacity (Variables|/Game/On_Mushrooms/Widgets/w_PickupText.w_PickupText_C|GetNameText _asw_pickup_text) (Utilities|Struct|MakeSlateColor (Utilities|Select :Index _humor :NewEnumerator0 "(R=0.870544,G=1.000000,B=0.076933,A=1.000000)" :NewEnumerator1 "(R=1.000000,G=0.554167,B=0.971598,A=1.000000)" :NewEnumerator2 "(R=0.000000,G=0.015345,B=0.291667,A=1.000000)" :NewEnumerator3 "(R=1.000000,G=0.000000,B=0.000000,A=1.000000)" :NewEnumerator4 "(R=1.000000,G=1.000000,B=1.000000,A=1.000000)")) :!class /Script/UMG.TextBlock))
    (:CastFailed
      _))
  (return))