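; Stamina consumable item that restores the top-down character's stamina when used from the inventory.
; On use, it checks stamina through the Cage's character reference; below maximum, it adds one point and has the Cage remove one item at its index.
; The actor destroys itself in either case, but at full stamina it leaves the Cage entry untouched.
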(event EventBeginPlay
  (|CallParentFunction) ; This node is disabled and will not be called.\nDrag off pins to build functionality.
)

(event Collision|EventActorBeginOverlap
  (params (OtherActor :type Actor%20Object%20Reference))
  (|CallParentFunction OtherActor) ; This node is disabled and will not be called.\nDrag off pins to build functionality.
)

(event EventTick
  (params (DeltaSeconds :type Float%20%28single-precision%29))
  (|CallParentFunction DeltaSeconds) ; This node is disabled and will not be called.\nDrag off pins to build functionality.
)

(event EventEventonUsed
  (bind _cage (Variables|Default|GetCage))
  (bind _topdowncharreference (Variables|/Game/On_Mushrooms/Blueptints/UI/bp_Cage.bp_Cage_C|GetTopDownCharReference _cage))
  (if (< (Variables|/Game/On_Mushrooms/Character/My_TopDownCharacter.My_TopDownCharacter_C|GetCurrentStamina _topdowncharreference) (Variables|/Game/On_Mushrooms/Character/My_TopDownCharacter.My_TopDownCharacter_C|GetMaxStamina _topdowncharreference))
    (Default|-IncreaseStamina _topdowncharreference 1)
    (Default|-RemoveItematIndex (Variables|Default|GetCage) (Variables|Default|GetIndex) 1 false)
    (Actor|DestroyActor) ; теперь он уничтожает иконку в инвентаре
    (else
      (Actor|DestroyActor) ; что оно делает?
    )))

(fn ConstructionScript
  (|CallParentFunction))