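; Master mushroom actor that drains the player character's stamina while they stand inside its sphere, if its humor matches the character's rolled cage humor.
; On overlap it compares the two humors once, showing a danger icon on a match.
; A Delay-driven loop then decreases stamina every second until end overlap clears the flag, hides the icon and sends a zero decrease.
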(event OnComponentBeginOverlap(Sphere)
  (params (OverlappedComponent :type Primitive%20Component%20Object%20Reference) (OtherActor :type Actor%20Object%20Reference) (OtherComp :type Primitive%20Component%20Object%20Reference) (OtherBodyIndex :type Integer) (bFromSweep :type Boolean) (SweepResult :type Hit%20Result%20Structure%20%28by%20ref%29))
  (Utilities|Casting|CastToMy_TopDownCharacter OtherActor)
  (Variables|Default|SetNotGetOver true)
  (bind _itisward (CallFunction|-ShowDangerIcon))
  (if _itisward :!label _label
    (if (stale OnComponentEndOverlap(Sphere) _output_get)
      (bind _output_get (Variables|Default|SetAmount 1))
      (Default|-DecreaseStamina (Variables|Default|GetTopDownCharacterReference) _output_get)
      (Utilities|FlowControl|Delay 1.0)
      (goto _label)
      (else
        _)))
  (bind _output_get_2 (Variables|Default|SetAmount 0))
  (Default|-DecreaseStamina (Variables|Default|GetTopDownCharacterReference) _output_get_2))

(event OnComponentEndOverlap(Sphere)
  (params (OverlappedComponent :type Primitive%20Component%20Object%20Reference) (OtherActor :type Actor%20Object%20Reference) (OtherComp :type Primitive%20Component%20Object%20Reference) (OtherBodyIndex :type Integer))
  (Utilities|Casting|CastToMy_TopDownCharacter OtherActor)
  (Rendering|SetVisibility (Variables|Default|GetDangerIcon) false true)
  (bind _output_get (Variables|Default|SetNotGetOver false))
  (bind _output_get_2 (Variables|Default|SetAmount 0))
  (Default|-DecreaseStamina (Variables|Default|GetTopDownCharacterReference) _output_get_2))

(event EventBeginPlay
  (bind _outactors (Actor|GetAllActorsOfClass "/Game/On_Mushrooms/Character/My_TopDownCharacter.My_TopDownCharacter_C"))
  (Variables|Default|SetTopDownCharacterReference (Utilities|Array|Get(acopy) _outactors)))

(event Collision|EventActorBeginOverlap
  (params (OtherActor :type Actor%20Object%20Reference)))

(fn ConstructionScript)

(fn -ShowDangerIcon
  (if (Utilities|Enum|Equal(Enum) (Variables|/Game/On_Mushrooms/Blueptints/UI/bp_Cage.bp_Cage_C|GetRolledHumor (Variables|/Game/On_Mushrooms/Character/My_TopDownCharacter.My_TopDownCharacter_C|GetCageRef (Variables|Default|GetTopDownCharacterReference))) (Utilities|Struct|Breaks_MushroomInfo (Variables|Default|GetMushroomInfo)))
    (Rendering|SetVisibility (Variables|Default|GetDangerIcon) true true)
    (return true)
    (else
      (Rendering|SetVisibility (Variables|Default|GetDangerIcon) false true)
      (return false))))