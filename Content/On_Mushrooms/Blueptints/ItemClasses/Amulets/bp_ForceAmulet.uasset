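; Force amulet item Blueprint that raises the overloaded cap on its referenced cage while equipped.
; On use, it asks the top-down character to equip it and, if that succeeds, increases the cap by its configured amount.
; StopInfluence subtracts the same amount, and both paths then refresh the cage's overloaded cap.
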(event EventBeginPlay
  (|CallParentFunction) ; This node is disabled and will not be called.\nDrag off pins to build functionality.
)

(event Collision|EventActorBeginOverlap
  (params (OtherActor :type Actor%20Object%20Reference))
  (|CallParentFunction OtherActor) ; This node is disabled and will not be called.\nDrag off pins to build functionality.
)

(event EventTick
  (params (DeltaSeconds :type Float%20%28single-precision%29))
  (|CallParentFunction DeltaSeconds) ; This node is disabled and will not be called.\nDrag off pins to build functionality.
)

(event EventEventonUsed
  (bind _cage_ref (Variables|Default|GetCage%20Ref))
  (bind _success (Default|-EquipAmulet (Variables|/Game/On_Mushrooms/Blueptints/UI/bp_Cage.bp_Cage_C|GetTopDownCharReference _cage_ref) self))
  (if _success
    (Default|-IncreaseOverloadedCap _cage_ref (Variables|Default|GetOverloadedCupAmountForAmulet))
    (Default|-UpdateOverloadedCap _cage_ref)))

(event EventStopInfluence
  (bind _cage_ref (Variables|Default|GetCage%20Ref))
  (Default|-DecreaseOverloadedCap _cage_ref (Variables|Default|GetOverloadedCupAmountForAmulet))
  (Default|-UpdateOverloadedCap _cage_ref))

(fn ConstructionScript
  (|CallParentFunction))